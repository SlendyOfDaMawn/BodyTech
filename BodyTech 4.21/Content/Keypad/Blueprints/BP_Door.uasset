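; Interactive door actor with configurable frame and door meshes that can start locked and be opened or closed with F.
; Tick enables input only while the player character's ItemName matches the door mesh's display name.
; F or OpenDoor toggles a timeline rotation with sound, or plays a guarded rattle animation if locked.
; UnlockDoor clears the lock and optionally opens the door automatically.
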(event `self.ReceiveBeginPlay`
  ;[1 1 1] Event Begin Play. Gets a reference to the player character
  (bind _asfirst_person_character (cast `/Game/Padlock/FirstPersonBP/Blueprints/FirstPersonCharacter` (`GameplayStatics.GetPlayerCharacter` 0)))
  (set `self.CharacterReference` _asfirst_person_character))

(event `self.ReceiveTick`
  (params (DeltaSeconds :type "Float (single-precision)"))
  ;[1 1 1] Event Tick. Enables/Disables Input
  (if (`KismetStringLibrary.EqualEqual_StrStr` (`KismetSystemLibrary.GetDisplayName` (`self.SM_Door`)) (`/Game/Padlock/FirstPersonBP/Blueprints/FirstPersonCharacter.ItemName` (`self.CharacterReference`)))
    (`self.EnableInput` (`GameplayStatics.GetPlayerController` 0))
    (else
      (`self.DisableInput` (`GameplayStatics.GetPlayerController` 0)))))

(event `UnlockDoor`
  ;[1 1 1] Unlocks the door
  (set `self.Locked?` false)
  (if (`self.OpenDoorAutomatically?`)
    (`self.OpenDoor`)))

(event `Key|F`
  (params (Key :type "Key Structure" :default "AnyKey"))
  (bind _dooropensoundcue (`self.DoorOpenSoundCue`))
  (bind _returnvalue (`SceneComponent.K2_GetComponentLocation` (`self.SM_Door`)))
  ;[1 1 1] Opens the door
  (:`Pressed`
    (if (`self.Locked?`) :!label _label
      (`self.DoorRattle`)
      (elif (`self.IsDoorOpen?`)
        (set `self.IsDoorOpen?` false)
        (`GameplayStatics.PlaySoundAtLocation` _dooropensoundcue _returnvalue)
        (bind (_direction _open_closedoor) (`Timeline|Open/CloseDoor` :!via `Reverse` :!label _label_2)
          (:`Update`
            (`SceneComponent.K2_SetRelativeRotation` (`self.SM_Door`) (`KismetMathLibrary.RLerp` (`self.DoorStartingRotation`) (`self.DoorEndingRotation`) _open_closedoor) false false)))
        (else
          (set `self.IsDoorOpen?` true)
          (`GameplayStatics.PlaySoundAtLocation` _dooropensoundcue _returnvalue)
          (goto _label_2))))))

(event `OpenDoor`
  ;[1 1 1] Opens the door
  (goto _label))

(event `DoorRattle`
  (bind (_doorstartingrotation_roll _doorstartingrotation_pitch) (`KismetMathLibrary.BreakRotator` (`self.DoorStartingRotation`)))
  ;[1 1 1] Rattle animation that plays when the player tries to open the door when it is locked
  (if (not (`self.RattleAnimationPlaying?`))
    (set `self.RattleAnimationPlaying?` true)
    (`GameplayStatics.PlaySoundAtLocation` (`self.DoorRattleSoundCue`) (`SceneComponent.K2_GetComponentLocation` (`self.SM_Door`)))
    (bind (_direction _rattle) (`Timeline|DoorRattleAnim` :!via `PlayFromStart`)
      (:`Update`
        (`SceneComponent.K2_SetRelativeRotation` (`self.SM_Door`) (`KismetMathLibrary.RLerp` (`self.DoorStartingRotation`) (`KismetMathLibrary.MakeRotator` _doorstartingrotation_roll _doorstartingrotation_pitch 0.5) _rattle) false false))
      (:`Finished`
        (set `self.RattleAnimationPlaying?` false)))))

(fn `UserConstructionScript`
  ;[1 1 1] Sets the static meshes chosen by the user
  (`StaticMeshComponent.SetStaticMesh` (`self.SM_DoorFrame`) (`self.DoorFrameMesh`))
  (`StaticMeshComponent.SetStaticMesh` (`self.SM_Door`) (`self.DoorMesh`))
  (set `self.DoorStartingRotation` (`SceneComponent.RelativeRotation` (`self.SM_Door`))))