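; Interactive keypad actor that unlocks every BP_Door whose name matches DoorNameToControl when the correct code is entered.
; Tick enables input while the character's ItemName matches a keypad part or it is in use; F or right-click toggles a close-up camera and cursor.
; Left-click traces tagged keys, animates them and reads digits from component names.
; EnterCode checks the fixed or construction-randomized code, flashing a light and playing a buzzer.
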(event `AnimateKey`
  ;[1 1 1] Animates the key moving. It first gets the relative location of the button and animate it being pressed.
  (if (not (`self.AnimationPlaying?`))
    (bind _output_get (set `self.StartLocation` (`SceneComponent.RelativeLocation` (`self.ClickedKey`))))
    (set `self.EndLocation` (`KismetMathLibrary.MakeVector` (.x _output_get) -0.1 (.z _output_get)))
    (bind (_direction _pressanimation) (`Timeline|AnimateKeyPress` :!via `PlayFromStart`)
      (:`Update`
        (`SceneComponent.K2_SetRelativeLocation` (`self.ClickedKey`) (`KismetMathLibrary.VLerp` (`self.StartLocation`) (`self.EndLocation`) _pressanimation) false false)
        (set `self.AnimationPlaying?` true))
      (:`Finished`
        (set `self.AnimationPlaying?` false)))))

(event `self.ReceiveBeginPlay`
  ;[1 1 1] Event Begin Play. Gets a reference to the First Person Character and sets it as a variable
  (bind _asfirst_person_character (cast `/Game/Padlock/FirstPersonBP/Blueprints/FirstPersonCharacter` (`GameplayStatics.GetPlayerCharacter` 0)))
  (set `self.CharacterReference` _asfirst_person_character))

(event `self.ReceiveTick`
  (params (DeltaSeconds :type "Float (single-precision)"))
  (bind _returnvalue (`GameplayStatics.GetPlayerController` 0))
  ;[1 1 1] Event Tick. Enables input to the keypad while the player is using it.
  (if (`KismetArrayLibrary.Array_Contains` (`self.KeypadNamesArray`) (`/Game/Padlock/FirstPersonBP/Blueprints/FirstPersonCharacter.ItemName` (`self.CharacterReference`)))
    (`self.EnableInput` _returnvalue :!label _label)
    (`WidgetBlueprintLibrary.SetInputMode_GameOnly` _returnvalue)
    (elif (`self.UsingKeypad?`)
      (goto _label)
      (else
        (`self.DisableInput` _returnvalue)))))

(event `Key|LeftMouseButton`
  (params (Key :type "Key Structure" :default "AnyKey"))
  (bind (_hitresult _returnvalue) (`PlayerController.GetHitResultUnderCursorForObjects` (`GameplayStatics.GetPlayerController` 0) (`|MakeArray` "ObjectTypeQuery1" "ObjectTypeQuery2" :!type "EObjectTypeQuery Enum") true))
  (bind _returnvalue_2 (`SceneComponent.K2_GetComponentLocation` (`self.Keypad`)))
  (bind (_bblockinghit _binitialoverlap _time _location _impactpoint _normal _impactnormal _physmat _hitactor _hitcomponent) (`GameplayStatics.BreakHitResult` _hitresult))
  (bind _returnvalue_3 (`KismetSystemLibrary.GetObjectName` _hitcomponent))
  ;[1 1 1] This is called when the player clicks on a button. It finds which button is pressed then eother enters the code, clears the entered code or adds the number to an array
  (:`Pressed`
    (if (and _returnvalue (`ActorComponent.ComponentHasTag` _hitcomponent "Key"))
      (set `self.ClickedKey` _hitcomponent)
      (`self.AnimateKey`)
      (`GameplayStatics.PlaySoundAtLocation` (`self.KeyPressSoundCue`) (`SceneComponent.K2_GetComponentLocation` (`self.Keypad`)))
      (switch `string` _returnvalue_3
        (:`Default`
          (`KismetArrayLibrary.Array_Add` (`self.EnteredCode`) (`KismetStringLibrary.Conv_StringToInt` _returnvalue_3))
          (if (and (== (`KismetArrayLibrary.Array_Length` (`self.EnteredCode`)) (`self.CodeLength`)) (`self.AutomaticallyEnderCode`))
            (for _array_element (`self.EnteredCode`) :!label _label_2
              (set `self.CodeString` (`KismetStringLibrary.Concat_StrStr` (`self.CodeString`) (`KismetStringLibrary.Conv_IntToString` _array_element))))
            (if (and (`KismetStringLibrary.EqualEqual_StrStr` (`self.Code`) (`self.CodeString`)) (<= (`KismetArrayLibrary.Array_Length` (`self.EnteredCode`)) (`self.CodeLength`)))
              (`self.ClearCode`)
              (`PrimitiveComponent.SetMaterial` (`self.Keypad`) 0 (`self.KeypadMaterialRight`))
              (`KismetSystemLibrary.Delay` 0.2)
              (`MaterialInstanceDynamic.SetScalarParameterValue` (`self.KeypadMaterialRight`) "Emmisivestrength" 150.0)
              (`GameplayStatics.PlaySoundAtLocation` (`self.BuzzerRightSoundCue`) _returnvalue_2)
              (`KismetSystemLibrary.Delay` 0.54)
              (`MaterialInstanceDynamic.SetScalarParameterValue` (`self.KeypadMaterialRight`) "Emmisivestrength" 0.0)
              (if (not (`self.CorrectCode?`))
                (set `self.CorrectCode?` true)
                (`self.ZoomOut`)
                (if (`self.CorrectCode?`) :!label _label_3
                  (bind _outactors (`GameplayStatics.GetAllActorsOfClass` "/Game/Keypad/Blueprints/BP_Door.BP_Door_C"))
                  (for _array_element_2 _outactors
                    (if (== (`/Game/Keypad/Blueprints/BP_Door.DoorName` _array_element_2) (`self.DoorNameToControl`))
                      (`/Game/Keypad/Blueprints/BP_Door.UnlockDoor` _array_element_2)))))
              (else
                (`self.ClearCode`)
                (`PrimitiveComponent.SetMaterial` (`self.Keypad`) 0 (`self.KeypadMaterialWrong`))
                (`KismetSystemLibrary.Delay` 0.2)
                (`MaterialInstanceDynamic.SetScalarParameterValue` (`self.KeypadMaterialWrong`) "Emmisivestrength" 150.0)
                (`GameplayStatics.PlaySoundAtLocation` (`self.BuzzerWrongSoundCue`) _returnvalue_2)
                (`KismetSystemLibrary.Delay` 0.54)
                (`MaterialInstanceDynamic.SetScalarParameterValue` (`self.KeypadMaterialWrong`) "Emmisivestrength" 0.0)
                (set `self.CorrectCode?` false)
                (goto _label_3)))))
        (:`Enter`
          (goto _label_2))
        (:`Clear`
          (`self.ClearCode`))))))

(event `Key|F`
  (params (Key :type "Key Structure" :default "AnyKey"))
  ;[1 1 1] When the player interacts with the keypad the camera zooms up close and enables the cursor. This allows the player to click on the buttons. If they press the same button again the opposite will happen
  (:`Pressed`
    (if (`self.UsingKeypad?`) :!label _label_4
      (`self.ClearCode`)
      (set `self.UsingKeypad?` false)
      (set `/Game/Padlock/FirstPersonBP/Blueprints/FirstPersonCharacter.UsingItem?` false (`self.CharacterReference`))
      (`PlayerController.SetViewTargetWithBlend` (`GameplayStatics.GetPlayerController` 0) (`self.CharacterReference`) 0.5 "VTBlend_Linear" 0.0 false)
      (set `PlayerController.bShowMouseCursor` false (`GameplayStatics.GetPlayerController` 0))
      (`WidgetBlueprintLibrary.SetInputMode_GameOnly` (`GameplayStatics.GetPlayerController` 0))
      (else
        (set `self.UsingKeypad?` true)
        (set `/Game/Padlock/FirstPersonBP/Blueprints/FirstPersonCharacter.UsingItem?` true (`self.CharacterReference`))
        (`PlayerController.SetViewTargetWithBlend` (`GameplayStatics.GetPlayerController` 0) self 0.5 "VTBlend_Linear" 0.0 false)
        (set `PlayerController.bShowMouseCursor` true (`GameplayStatics.GetPlayerController` 0))))))

(event `ZoomOut`
  ;[1 1 1] When the player interacts with the keypad the camera zooms up close and enables the cursor. This allows the player to click on the buttons. If they press the same button again the opposite will happen
  (goto _label_4))

(event `Key|RightMouseButton`
  (params (Key :type "Key Structure" :default "AnyKey"))
  ;[1 1 1] When the player interacts with the keypad the camera zooms up close and enables the cursor. This allows the player to click on the buttons. If they press the same button again the opposite will happen
  (:`Pressed`
    (goto _label_4)))

(fn `ClearCode`
  ;[1 1 1] Resets the code when the clear button is pressed
  (`KismetArrayLibrary.Array_Clear` (`self.EnteredCode`))
  (set `self.CodeString` "")
  (return))

(fn `UserConstructionScript`
  ;[1 1 1] Creates a dynamic material for the right/wrong light
  (bind _returnvalue (`PrimitiveComponent.CreateDynamicMaterialInstance` (`self.Keypad`) 0 "/Game/Keypad/Materials/M_Keypad_Red.M_Keypad_Red"))
  (set `self.KeypadMaterialWrong` _returnvalue)
  (bind _returnvalue_2 (`PrimitiveComponent.CreateDynamicMaterialInstance` (`self.Keypad`) 0 "/Game/Keypad/Materials/M_Keypad_Green.M_Keypad_Green"))
  (set `self.KeypadMaterialRight` _returnvalue_2)
  ;[1 1 1] Sets the transform of the camera
  (`SceneComponent.K2_AddLocalTransform` (`self.Camera`) (`self.CameraTransform`) false false)
  ;[1 1 1] Sets a random code
  (if (`self.RandomCode?`)
    (set `self.Code` (`KismetStringLibrary.Conv_IntToString` (`KismetMathLibrary.RandomIntegerInRange` 1000 9999)))
    (set `self.CodeLength` 4)
    (else
      (set `self.CodeLength` (`KismetStringLibrary.Len` (`self.Code`)))))
  (if (`self.TurnOffText?`)
    (`SceneComponent.SetHiddenInGame` (`self.TextRender`) true false)
    (else
      (`TextRenderComponent.K2_SetText` (`self.TextRender`) (`KismetTextLibrary.Conv_StringToText` (`self.Code`)))))
  (for (_array_element _array_index) (`|MakeArray` (`self.Keypad`) (`self.0`) (`self.1`) (`self.2`) (`self.3`) (`self.4`) (`self.5`) (`self.6`) (`self.7`) (`self.8`) (`self.9`) (`self.Clear`) (`self.Enter`))
    (`KismetArrayLibrary.Array_Set` (`self.KeypadNamesArray`) _array_index (`KismetSystemLibrary.GetDisplayName` _array_element) true)))