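; Scene component that projects a ScanFX laser beam along its forward vector.
; On BeginPlay it attaches a beam emitter to itself and applies the laser material.
; Each tick a visibility line trace, ignoring the owner, sets the beam end to the impact point or the maximum trace distance.
; A one-time material reapply on first tick works around spawn-exposed parameters not being ready during BeginPlay.
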(event `self.ReceiveBeginPlay`
  ;[0.1 0.1 0.1] Create a beam particle system and apply laser material to it.
  (bind _returnvalue (`GameplayStatics.SpawnEmitterAttached` "/Game/ScanFX/Particles/P_ScanFX_LaserBeam.P_ScanFX_LaserBeam" self "None" (0.0 0.0 0.0) (struct) "SnapToTarget" false))
  (bind _output_get (set `self.Laser Emitter` _returnvalue))
  (`PrimitiveComponent.SetMaterial` _output_get 0 (`self.Laser Material`)))

(event `self.ReceiveTick`
  (params (DeltaSeconds :type "Float (single-precision)"))
  (bind _returnvalue (`self.K2_GetComponentLocation`))
  (bind _returnvalue_2 (+ _returnvalue (* (`self.GetForwardVector`) (`self.Trace Distance`))))
  (`|ExecutionSequence`
    (:`then_0`
      ;[0.1 0.1 0.1] Trace for blocking visibility along the lasers path
      (bind (_outhit _returnvalue_3) (`KismetSystemLibrary.LineTraceSingle` _returnvalue _returnvalue_2 "TraceTypeQuery1" true (`|MakeArray` (`self.GetOwner`))))
      ;[0.1 0.1 0.1] Set the laser beam to end at impact or if no impact occured at the end of the trace distance
      (`ParticleSystemComponent.SetBeamTargetPoint` (`self.Laser Emitter`) 0 (`KismetMathLibrary.SelectVector` (`.Location` (`GameplayStatics.BreakHitResult` _outhit)) _returnvalue_2 _returnvalue_3) 0))
    (:`then_1`
      ;[0.1 0.1 0.1] Parameters exposed on spawn do not get recognized during BeginPlay so this fixes a missing material if the ocmponent is spawned
      (`/Engine/EditorBlueprintResources/StandardMacros.DoOnce` false
        (:`Completed`
          (`PrimitiveComponent.SetMaterial` (`self.Laser Emitter`) 0 (`self.Laser Material`)))))))