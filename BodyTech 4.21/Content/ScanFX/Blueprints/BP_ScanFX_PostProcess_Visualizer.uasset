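; Post-process visualizer actor for ScanFX that applies configured post-process settings and a scan material, built entirely in the construction script.
; It sizes and centers a box from two corner points, then creates a post-process component attached to that box.
; When a parent material is valid, it adds a dynamic instance as a blendable, passing the actor's location as the scan start point.
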(fn `UserConstructionScript`
  (bind _material_parent (`self.Material Parent`))
  (bind _bottom_corner (`self.Bottom Corner`))
  (bind _top_corner (`self.Top Corner`))
  (`|ExecutionSequence`
    (:`then_0`
      ;[0.1 0.1 0.1] Fit the box to the configured size
      (`BoxComponent.SetBoxExtent` (`self.Box`) (* (- _top_corner _bottom_corner) 0.5) true)
      (`SceneComponent.K2_SetRelativeLocation` (`self.Box`) (* (+ _top_corner _bottom_corner) 0.5) false false))
    (:`then_1`
      ;[0.1 0.1 0.1] Create post process component and set configured settings.
      (bind _returnvalue (`AddComponent|Post Process Component_1`))
      (bind _output_get (set `self.Post Process Component` _returnvalue))
      (`SceneComponent.K2_AttachToComponent` _output_get (`self.Box`) "None" "KeepRelative" "KeepRelative" "KeepRelative" true)
      (set `PostProcessComponent.Settings` (`self.PP Settings`) _output_get))
    (:`then_2`
      ;[0.1 0.1 0.1] Create material instance and apply as blendable
      (`/Engine/EditorBlueprintResources/StandardMacros.IsValid` _material_parent
        (:`Is Valid`
          (bind _returnvalue_2 (`KismetMaterialLibrary.CreateDynamicMaterialInstance` _material_parent))
          (bind _output_get_2 (set `self.MID` _returnvalue_2))
          (`MaterialInstanceDynamic.SetVectorParameterValue` _output_get_2 "Scan Start Location" (`KismetMathLibrary.Conv_VectorToLinearColor` (`self.K2_GetActorLocation`)))
          (`PostProcessComponent.AddOrUpdateBlendable` (`self.Post Process Component`) _output_get_2 1.0))))))